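; Lockpicking minigame actor that takes over player input and shows itself through a capture-fed widget until success, failure or exit.
; MouseX angles the pick toward a random target; holding Lockpick turns the lock if within tolerance, otherwise jiggles it and drains pick health.
; Looping timers drive rotation, and broken picks fall with physics before replacement.
; A full turn unlocks and uses TargetDoor; running out of picks fails.
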(event `self.ReceiveBeginPlay`
  (`self.GenerateLock`)
  (add `self.OnLockpickSuccessful` (`|CreateDelegate` :!event `LockpickingSuccess`)))

(event `CreateLockpickingWidget`
  (bind _returnvalue (`GameplayStatics.GetPlayerController` 0))
  ;[1 1 1] Create lockpiking widget
  (`SceneCaptureComponent.ShowOnlyActorComponents` (`self.LockpickingCapture`) self false)
  (bind _returnvalue_2 (`|CreateWidget` "/Game/Lockpick/WB_LockpickingWidget.WB_LockpickingWidget_C" null self))
  (bind _output_get (set `self.WB_Lockpicking` _returnvalue_2))
  (`UserWidget.AddToViewport` _output_get 0)
  (`self.DisableInput` (`/Game/Lockpick/Mechanics/BPFL_UniveralFunctions.GetPlayer`) _returnvalue)
  (`self.EnableInput` _returnvalue))

(event `LockpickingFail`
  (bind _returnvalue (`GameplayStatics.GetPlayerController` 0))
  ;[1 1 1] Lockpicking Fail/End
  (`self.DisableInput` _returnvalue)
  (`self.EnableInput` (`/Game/Lockpick/Mechanics/BPFL_UniveralFunctions.GetPlayer`) _returnvalue)
  (bind _wb_lockpicking (`self.WB_Lockpicking`)
    (:`then`
      (`Widget.RemoveFromParent` _wb_lockpicking)
      (set `self.WB_Lockpicking` null)
      (`self.K2_DestroyActor`))
    (:`else`)))

(event `LockpickingSuccess`
  ;[1 1 1] Lockpicking Success
  (`KismetSystemLibrary.K2_SetTimerDelegate` (delegate `LockpickingFinished`) 0.5)
  (set `self.LockComplete` true))

(event `LockpickingFinished`
  (bind _returnvalue (`GameplayStatics.GetPlayerController` 0))
  ;[1 1 1] Lockpicking Success
  (`self.DisableInput` _returnvalue)
  (`self.EnableInput` (`/Game/Lockpick/Mechanics/BPFL_UniveralFunctions.GetPlayer`) _returnvalue)
  (bind _wb_lockpicking (`self.WB_Lockpicking`)
    (:`then`
      (`Widget.RemoveFromParent` _wb_lockpicking)
      (set `self.WB_Lockpicking` null)
      (bind _targetdoor (`self.TargetDoor`)
        (:`then`
          (`/Game/Lockpick/BP_Door.UseDoor` _targetdoor)
          (set `/Game/Lockpick/BP_Door.IsLocked` false _targetdoor)
          (`self.K2_DestroyActor`))
        (:`else`)))
    (:`else`)))

(event `EnhancedInput|/Game/FirstPerson/Input/Actions/IA_Interact`
  (params (ActionValue :type Boolean) (ElapsedSeconds :type "Float (double-precision)") (TriggeredSeconds :type "Float (double-precision)") (InputAction :type "InputAction Object Reference" :default "/Game/FirstPerson/Input/Actions/IA_Interact.IA_Interact"))
  (:`Started`
    (`self.LockpickingFail`)))

(event `InputAxisKey|MouseX`
  (params (AxisValue :type "Float (single-precision)"))
  (bind (_returnvalue_roll _returnvalue_pitch _returnvalue_yaw) (`KismetMathLibrary.BreakRotator` (`KismetMathLibrary.ComposeRotators` (`SceneComponent.RelativeRotation` (`self.LockpickRotationScene`)) (`KismetMathLibrary.MakeRotator` (* AxisValue -3.0)))))
  ;[1 1 1] Lockpick rotation x-axis
  (if (not (`self.IsLockRotating`))
    (bind _output_get (set `self.LockpickRotation` (`KismetMathLibrary.FClamp` _returnvalue_roll -90.0 90.0)))
    (`SceneComponent.K2_SetRelativeRotation` (`self.LockpickRotationScene`) (`KismetMathLibrary.MakeRotator` _output_get _returnvalue_pitch _returnvalue_yaw) false false)))

(event `ForwardLockRotation`
  ;[1 1 1] forwward
  (`KismetSystemLibrary.K2_PauseTimerHandle` (`self.BackwardLockTimer`))
  (bind _returnvalue (`KismetSystemLibrary.K2_SetTimerDelegate` (delegate `UpdateForwardLockRotation`) 0.02 true))
  (set `self.ForwardLockTimer` _returnvalue)
  (`KismetSystemLibrary.K2_PauseTimerHandle` (`self.JammedLock`)))

(event `UpdateForwardLockRotation`
  (bind (_returnvalue_roll _returnvalue_pitch _returnvalue_yaw) (`KismetMathLibrary.BreakRotator` (`KismetMathLibrary.ComposeRotators` (`SceneComponent.RelativeRotation` (`self.LockRotationScene`)) (`KismetMathLibrary.MakeRotator` (- 0.0 3.0)))))
  ;[1 1 1] forwward
  (if (`self.IsLockRotating`)
    (bind _output_get (set `self.LockRotation` (`KismetMathLibrary.FClamp` _returnvalue_roll -90.0 0.0)))
    (`SceneComponent.K2_SetRelativeRotation` (`self.LockRotationScene`) (`KismetMathLibrary.MakeRotator` _output_get _returnvalue_pitch _returnvalue_yaw) false false)
    (`self.LockpickForward`)
    (if (== (`self.LockRotation`) -90.0)
      (`KismetSystemLibrary.K2_PauseTimerHandle` (`self.ForwardLockTimer`))
      (`self.OnLockpickSuccessful`))))

(event `BackwordLockRotation`
  ;[1 1 1] backward lock rotation
  (`KismetSystemLibrary.K2_PauseTimerHandle` (`self.ForwardLockTimer`))
  (bind _returnvalue (`KismetSystemLibrary.K2_SetTimerDelegate` (delegate `UpdateBackwardLockRotation`) 0.02 true))
  (set `self.BackwardLockTimer` _returnvalue))

(event `UpdateBackwardLockRotation`
  (bind (_returnvalue_roll _returnvalue_pitch _returnvalue_yaw) (`KismetMathLibrary.BreakRotator` (`KismetMathLibrary.ComposeRotators` (`SceneComponent.RelativeRotation` (`self.LockRotationScene`)) (`KismetMathLibrary.MakeRotator` (+ 0.0 6.0)))))
  ;[1 1 1] backward lock rotation
  (if (not (`self.IsLockRotating`))
    (bind _output_get (set `self.LockRotation` (`KismetMathLibrary.FClamp` _returnvalue_roll -90.0 0.0)))
    (`SceneComponent.K2_SetRelativeRotation` (`self.LockRotationScene`) (`KismetMathLibrary.MakeRotator` _output_get _returnvalue_pitch _returnvalue_yaw) false false)
    (`self.LockpickBackward`)
    (if (== (`self.LockRotation`) 0.0)
      (`KismetSystemLibrary.K2_PauseTimerHandle` (`self.BackwardLockTimer`)))))

(event `EnhancedInput|/Game/FirstPerson/Input/Actions/IA_Lockpick`
  (params (ActionValue :type Boolean) (ElapsedSeconds :type "Float (double-precision)") (TriggeredSeconds :type "Float (double-precision)") (InputAction :type "InputAction Object Reference" :default "/Game/FirstPerson/Input/Actions/IA_Lockpick.IA_Lockpick"))
  ;[1 1 1] Lockpick
  (:`Started`
    (set `self.IsLockRotating` true)
    (if (`self.CheckUnlockStatus`)
      (`self.ForwardLockRotation`)
      (else
        (`self.LockJammed`))))
  (:`Completed`
    (set `self.IsLockRotating` false)
    (if (not (`self.LockComplete`))
      (`self.BackwordLockRotation`))))

(event `LockJammed`
  ;[1 1 1] Jammed Lock Rotation
  (bind _returnvalue (`KismetSystemLibrary.K2_SetTimerDelegate` (delegate `UpdateJammedLock`) 0.02 true))
  (set `self.JammedLock` _returnvalue))

(event `UpdateJammedLock`
  (bind (_returnvalue_roll _returnvalue_pitch _returnvalue_yaw) (`KismetMathLibrary.BreakRotator` (`KismetMathLibrary.ComposeRotators` (`SceneComponent.RelativeRotation` (`self.LockRotationScene`)) (`KismetMathLibrary.MakeRotator` (`self.JammedValue`)))))
  ;[1 1 1] Jammed Lock Rotation
  (if (`self.IsLockRotating`)
    (`|ExecutionSequence`
      (:`then_0`
        (`/Engine/EditorBlueprintResources/StandardMacros.FlipFlop`
          (:`A`
            (set `self.JammedValue` -3.0))
          (:`B`
            (set `self.JammedValue` 3.0))))
      (:`then_1`
        (bind _output_get (set `self.LockRotation` (`KismetMathLibrary.FClamp` _returnvalue_roll -6.0 0.0)))
        (`SceneComponent.K2_SetRelativeRotation` (`self.LockRotationScene`) (`KismetMathLibrary.MakeRotator` _output_get _returnvalue_pitch _returnvalue_yaw) false false)
        (`self.LockpickHealth`)))))

(event `LockpickHealth`
  ;[1 1 1] breaking lockspick
  (bind _output_get (set `self.TrackLockpickHealth` (`KismetMathLibrary.FClamp` (- (`self.TrackLockpickHealth`) 4.0) 0.0 100.0)))
  (if (<= _output_get 0.0)
    (`/Engine/EditorBlueprintResources/StandardMacros.DoOnce` false :!label _label
      (:`Completed`
        (bind _result (`/Engine/EditorBlueprintResources/StandardMacros.DecrementInt` (`/Game/FirstPerson/Blueprints/BP_FirstPersonCharacter.Lockpicks` (`/Game/Lockpick/Mechanics/BPFL_UniveralFunctions.GetPlayer`)))
          (:`  `
            (`self.OnLockpickBroken` _result)
            (add `self.OnLockpickBroken` (delegate `NoMoreLockpicks`))
            (if (> (`/Game/FirstPerson/Blueprints/BP_FirstPersonCharacter.Lockpicks` (`/Game/Lockpick/Mechanics/BPFL_UniveralFunctions.GetPlayer`)) 0)
              (`self.LockpicksAnim`)
              (`self.NewLockpick`))))))))

(event `ResettLockpick`
  ;[1 1 1] breaking lockspick
  (goto _label :!via `Reset`))

(event `NoMoreLockpicks` :!signature `self.OnLockpickBroken`
  (params (Lockpicks :type Integer))
  ;[1 1 1] breaking lockspick
  (if (<= Lockpicks 0)
    (`self.LockpickingFail`)))

(event `LockpicksAnim`
  (bind _lockpickbroken1 (`self.LockpickBroken1`))
  ;[1 1 1] Lockpick Anim
  (`SceneComponent.SetVisibility` (`self.LockpickBroken`) true false)
  (`SceneComponent.SetVisibility` (`self.LockpickBroken1`) true false)
  (`SceneComponent.SetVisibility` (`self.Lockpick`) false false)
  (`PrimitiveComponent.SetSimulatePhysics` _lockpickbroken1 false)
  (`PrimitiveComponent.SetCollisionEnabled` _lockpickbroken1 "NoCollision")
  (`SceneComponent.K2_SetRelativeTransform` (`self.LockpickBroken1`) (`SceneComponent.GetRelativeTransform` (`self.LockpickBroken`)) false false)
  (`KismetSystemLibrary.K2_SetTimerDelegate` (delegate `BeginAnimation`) 0.1))

(event `BeginAnimation`
  (bind _lockpickbroken1 (`self.LockpickBroken1`))
  (bind _lockpickbroken1_2 (`self.LockpickBroken1`))
  ;[1 1 1] Lockpick Anim
  (`PrimitiveComponent.SetSimulatePhysics` _lockpickbroken1_2 true)
  (`PrimitiveComponent.SetCollisionEnabled` _lockpickbroken1_2 "QueryAndPhysics")
  (`KismetSystemLibrary.Delay` 1.0)
  (`PrimitiveComponent.SetSimulatePhysics` _lockpickbroken1 false)
  (`PrimitiveComponent.SetCollisionEnabled` _lockpickbroken1 "NoCollision"))

(event `NewLockpick`
  ;[1 1 1] add new lockpick
  (`KismetSystemLibrary.K2_SetTimerDelegate` (delegate `AddNewLockpick`) 1.0)
  (set `self.IsLockRotating` false)
  (`self.DisableInput` (`GameplayStatics.GetPlayerController` 0)))

(event `AddNewLockpick`
  ;[1 1 1] add new lockpick
  (`SceneComponent.SetVisibility` (`self.Lockpick`) true false)
  (`SceneComponent.SetVisibility` (`self.LockpickBroken`) false false)
  (`SceneComponent.SetVisibility` (`self.LockpickBroken1`) false false)
  (set `self.TrackLockpickHealth` 100.0)
  (`self.ResettLockpick`)
  (`self.EnableInput` (`GameplayStatics.GetPlayerController` 0)))

(fn `CheckUnlockStatus`
  (returns (Success :type Boolean))
  (return (`KismetMathLibrary.NearlyEqual_FloatFloat` (`self.LockpickRotation`) (`self.UnlockValue`) (`self.RandomTolerance`))))

(fn `GenerateLock`
  (bind _output_get (set `self.UnlockValue` (`KismetMathLibrary.RandomFloatInRange` -90.0 90.0)))
  (`KismetSystemLibrary.PrintString` (`KismetStringLibrary.Conv_DoubleToString` _output_get) true true (struct :`G` 0.66 :`B` 1.0 :`A` 1.0) 50.0))

(fn `LockpickBackward`
  (bind (_relativelocation_x _relativelocation_y _relativelocation_z) (`KismetMathLibrary.BreakVector` (`SceneComponent.RelativeLocation` (`self.LockpickRotationScene`))))
  (`SceneComponent.K2_SetRelativeLocation` (`self.LockpickRotationScene`) (`KismetMathLibrary.MakeVector` _relativelocation_x (`KismetMathLibrary.FClamp` (+ _relativelocation_y 0.32) -4.8 0.0) (`KismetMathLibrary.FClamp` (+ _relativelocation_z 0.2) 0.0 3.0)) false false))

(fn `LockpickForward`
  (bind (_relativelocation_x _relativelocation_y _relativelocation_z) (`KismetMathLibrary.BreakVector` (`SceneComponent.RelativeLocation` (`self.LockpickRotationScene`))))
  (`SceneComponent.K2_SetRelativeLocation` (`self.LockpickRotationScene`) (`KismetMathLibrary.MakeVector` _relativelocation_x (`KismetMathLibrary.FClamp` (- _relativelocation_y 0.16) -4.0 0.0) (`KismetMathLibrary.FClamp` (- _relativelocation_z 0.1) 0.0 100.0)) false false))

(fn `UserConstructionScript`)