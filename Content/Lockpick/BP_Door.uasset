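; Lockable door actor that swings open and closed on interaction and hands off to a lockpicking minigame when locked.
; UseDoor toggles IsOpen and plays or reverses a timeline that lerps the door mesh's yaw.
; If locked and the player has lockpicks, it spawns BP_Lockpicking_Actor far above the world origin with itself as TargetDoor, then has that actor create its lockpicking widget.
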(event `UseDoor`
  ;[1 1 1] open / close door
  (if (not (`self.IsOpen`))
    (set `self.IsOpen` true)
    (bind (_direction _dooropenning) (`Timeline|Timeline` :!label _label)
      (:`Update`
        (`SceneComponent.K2_SetRelativeRotation` (`self.Door`) (`KismetMathLibrary.MakeRotator` 0.0 0.0 (`KismetMathLibrary.Lerp` 0.0 100.0 _dooropenning)) false false)))
    (else
      (set `self.IsOpen` false)
      (goto _label :!via `Reverse`))))

(event `/Game/Lockpick/BPI_Interaction.InteractWith`
  (params (Interactor :type "Actor Object Reference"))
  (if (not (`self.IsLocked`))
    (`self.UseDoor`)
    (else
      (`KismetSystemLibrary.LogString` "Door Is locked" false)
      (`self.CreateLock`))))

(event `CreateLock`
  (if (`self.AnyLockpicks`)
    (bind _returnvalue (`|SpawnActorFromClass` "/Game/Lockpick/BP_Lockpicking_Actor.BP_Lockpicking_Actor_C" (`KismetMathLibrary.MakeTransform` (0.0 0.0 1000000.0)) "Undefined" "MultiplyWithRoot" null self null))
    (`/Game/Lockpick/BP_Lockpicking_Actor.CreateLockpickingWidget` _returnvalue)))

(fn `AnyLockpicks`
  (returns (ReturnValue :type Boolean))
  (return (not (<= (`/Game/FirstPerson/Blueprints/BP_FirstPersonCharacter.Lockpicks` (`/Game/Lockpick/Mechanics/BPFL_UniveralFunctions.GetPlayer`)) 0))))

(fn `UserConstructionScript`)