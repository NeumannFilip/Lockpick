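; Interaction component that finds an interactable actor near its owner and triggers it on player input.
; BeginPlay sets a non-looping 0.2-second timer for a debug-drawn sphere trace starting ahead of the owner, with no End set.
; The trace stores a hit actor implementing BPI_Interaction as TargetActor, otherwise clearing it.
; IA_Interact calls InteractWithMessage on a valid target, passing the owner.
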(event `self.ReceiveBeginPlay`
  (`self.BeginTrace`))

(event `BeginTrace`
  ;[1 0.5923 0.5724] trace interaction
  (`KismetSystemLibrary.K2_SetTimerDelegate` (delegate `UpdateTrace`) 0.2))

(event `UpdateTrace`
  ;[1 0.5923 0.5724] trace interaction
  (`self.InteractionTrace`))

(event `EnhancedInput|/Game/FirstPerson/Input/Actions/IA_Interact`
  (params (ActionValue :type Boolean) (ElapsedSeconds :type "Float (double-precision)") (TriggeredSeconds :type "Float (double-precision)") (InputAction :type "InputAction Object Reference" :default "/Game/FirstPerson/Input/Actions/IA_Interact.IA_Interact"))
  (:`Started`
    (bind _targetactor (`self.TargetActor`)
      (:`then`
        (message `/Game/Lockpick/BPI_Interaction.InteractWith` _targetactor (`self.GetOwner`)))
      (:`else`))))

(fn `InteractionTrace`
  (bind _returnvalue (`self.GetOwner`))
  (bind (_outhit _returnvalue_2) (`KismetSystemLibrary.SphereTraceSingle` :`Start` (+ (`Actor.K2_GetActorLocation` _returnvalue) (* (`Actor.GetActorForwardVector` _returnvalue) 150.0)) :`Radius` 70.0 :`TraceChannel` "TraceTypeQuery3" :`DrawDebugType` "ForDuration"))
  (if _returnvalue_2
    (bind (_bblockinghit _binitialoverlap _time _distance _location _impactpoint _normal _impactnormal _physmat _hitactor) (`GameplayStatics.BreakHitResult` _outhit))
    (if (`KismetSystemLibrary.DoesImplementInterface` _hitactor "/Game/Lockpick/BPI_Interaction.BPI_Interaction_C")
      (set `self.TargetActor` _hitactor)
      (else
        (set `self.TargetActor` null)))
    (else
      (set `self.TargetActor` null))))